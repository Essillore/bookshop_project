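; BPC_Inventory is an inventory component that adds and removes named items in a slot array.
; AddItem writes the item into the first slot holding "None", and RemoveItem resets the first matching slot to "None".
; Both functions then create a widget carrying the item name and add it to the viewport, with AddItem using UMG_InventoryUpdate flagged as an addition.
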(fn `AddItem`
  (params (ItemToAdd :type Name))
  (bind _inventoryslots (`self.InventorySlots`))
  (`KismetArrayLibrary.Array_Set` _inventoryslots (`KismetArrayLibrary.Array_Find` _inventoryslots) ItemToAdd)
  (bind _returnvalue (`|CreateWidget` "/Game/UMG/Inventory/UMG_InventoryUpdate.UMG_InventoryUpdate_C" null ItemToAdd true))
  (`UserWidget.AddToViewport` _returnvalue 0)
  (return))

(fn `RemoveItem`
  (params (ItemToRemove :type Name))
  (bind _inventoryslots (`self.InventorySlots`))
  (`KismetArrayLibrary.Array_Set` _inventoryslots (`KismetArrayLibrary.Array_Find` _inventoryslots ItemToRemove))
  (bind _returnvalue (`|CreateWidget` "/Game/UMG/Inventory/UMG_InventoryUpdate.UMG_InventoryUpdate_C" null ItemToRemove))
  (`UserWidget.AddToViewport` _returnvalue 0)
  (return))