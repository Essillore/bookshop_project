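; Base interactable object that acts as an audio player, pickup or inspectable, chosen by its ObjectType.
; The Interaction event stores the player and branches: toggle audio if a tape is loaded, add the item name to inventory and destroy itself, or inspect.
; Inspection passes the mesh to the level's BP_Inspect actor and opens the inspect UI with a mouse cursor.
; Highlight functions toggle the mesh's custom depth rendering.
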(event `/Game/Blueprints/Interfaces/BPI_InteractableObject.Interaction`
  (params (PlayerRef :type "/Game/FirstPerson/Blueprints/BP_FirstPersonCharacter Object Reference"))
  (bind _output_get (set `self.Player Ref` PlayerRef))
  (switch `/Game/Blueprints/Enum/Enum_ObjectType` (`self.ObjectType`)
    (:`NewEnumerator0`
      (`self.Audio Logic`))
    (:`NewEnumerator3`
      (`self.Pickup Object` _output_get))
    (:`NewEnumerator4`
      (`self.InspectObject`))))

(fn `Audio Logic`
  (locals (`TapeLoaded?` :type Boolean :default true))
  (bind _audio (`self.Audio`))
  (if (`local.TapeLoaded?`)
    (if (`AudioComponent.IsPlaying` _audio)
      (`AudioComponent.Stop` _audio)
      (else
        (`AudioComponent.Play` _audio 0.0)))))

(fn `GetType`
  (returns (ObjectType :type "/Game/Blueprints/Enum/Enum_ObjectType Enum"))
  (return (`self.ObjectType`)))

(fn `Hightlight`
  (returns (NewParam :type Boolean))
  (`PrimitiveComponent.SetRenderCustomDepth` (`self.MainMesh`) true)
  (return false))

(fn `InspectObject`
  (bind _returnvalue (`GameplayStatics.GetPlayerController` 0))
  (bind _player_ref (`self.Player Ref`))
  (bind _returnvalue_2 (`GameplayStatics.GetActorOfClass` "/Game/Blueprints/InspectSystem/BP_Inspect.BP_Inspect_C"))
  (`/Engine/EditorBlueprintResources/StandardMacros.IsValid` _returnvalue_2
    (:`Is Valid`
      (`/Game/Blueprints/InspectSystem/BP_Inspect.UpdateMesh` _returnvalue_2 (`StaticMeshComponent.StaticMesh` (`self.MainMesh`)) _player_ref)
      (bind _returnvalue_3 (`|CreateWidget` "/Game/Blueprints/InspectSystem/UMG_InspectUi.UMG_InspectUi_C" null (`KismetTextLibrary.Conv_NameToText` (`self.ObjectName`)) _player_ref))
      (`UserWidget.AddToViewport` _returnvalue_3 0)
      (`WidgetBlueprintLibrary.SetInputMode_GameAndUIEx` _returnvalue _returnvalue_3)
      (set `PlayerController.bShowMouseCursor` true _returnvalue))))

(fn `InspectTest`
  (bind _returnvalue (`GameplayStatics.GetPlayerCameraManager` 0))
  (`self.K2_SetActorLocation` (+ (`PlayerCameraManager.GetCameraLocation` _returnvalue) (* (`KismetMathLibrary.GetForwardVector` (`PlayerCameraManager.GetCameraRotation` _returnvalue)) 100.0)))
  (`self.K2_AttachToComponent` (`/Game/FirstPerson/Blueprints/BP_FirstPersonCharacter.HeldObjectLoc` (`self.Player Ref`)) "None" "KeepWorld" "SnapToTarget" "KeepRelative")
  (`PrimitiveComponent.SetSimulatePhysics` (`self.MainMesh`) false)
  (`PrimitiveComponent.SetCollisionEnabled` (`self.MainMesh`) "NoCollision"))

(fn `Pickup Object`
  (params (PlayerRef :type "/Game/FirstPerson/Blueprints/BP_FirstPersonCharacter Object Reference"))
  (`/Game/Blueprints/InventorySystem/BPC_Inventory.AddItem` (`/Game/FirstPerson/Blueprints/BP_FirstPersonCharacter.BPC_Inventory` PlayerRef) (`self.ObjectName`))
  (`/Engine/EditorBlueprintResources/StandardMacros.IsValid` self
    (:`Is Valid`
      (`self.K2_DestroyActor`))))

(fn `UnHighlight`
  (returns (NewParam :type Boolean))
  (`PrimitiveComponent.SetRenderCustomDepth` (`self.MainMesh`) false)
  (return false))

(fn `UserConstructionScript`)